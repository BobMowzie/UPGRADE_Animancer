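; An animation notify that spawns attack hitboxes for a ShujaaV3 character when the animation reaches it.
; It clears the owner's ActorsHit list, then spawns one Hitbox actor at the owner's transform for each entry in the notify's Hitboxes array.
; Each entry is passed to its actor as Data, and the spawned hitboxes are added to the character's own Hitboxes array.
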(fn `NewFunction_0`)

(fn `Received_Notify`
  (params (MeshComp :type "SkeletalMeshComponent Object Reference") (Animation :type "AnimSequenceBase Object Reference"))
  (returns (ReturnValue :type Boolean))
  (bind _asshujaa_v3 (cast `/Game/Characters/Shujaa3/ShujaaV3` (`ActorComponent.GetOwner` MeshComp)))
  (`BlueprintSetLibrary.Set_Clear` (`/Game/Characters/Shujaa3/ShujaaV3.ActorsHit` _asshujaa_v3))
  (for _array_element (`self.hitboxes`)
    (bind _returnvalue (`|SpawnActorFromClass` "/Game/Blueprints/Mechanics/hitbox.hitbox_C" (`Actor.GetTransform` _asshujaa_v3) "Undefined" "OverrideRootScale" null _array_element null))
    (`KismetArrayLibrary.Array_Add` (`/Game/Characters/Shujaa3/ShujaaV3.hitboxes` _asshujaa_v3) _returnvalue))
  (return false))