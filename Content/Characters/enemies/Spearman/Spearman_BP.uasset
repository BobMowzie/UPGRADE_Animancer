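; Spearman enemy character Blueprint that arms itself with a spear when play begins.
; BeginPlay runs the parent logic, then spawns a SpearActor and snaps its root component to the mesh's spear_socket.
; Tick and the construction script only call their parent versions, so the spear attachment is the only logic added in these graphs.
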(event `self.ReceiveBeginPlay`
  (`parent.ReceiveBeginPlay`)
  (bind _returnvalue (`|SpawnActorFromClass` "/Game/Characters/enemies/Spearman/SpearActor.SpearActor_C" (`self.GetTransform`) "Undefined" "OverrideRootScale" null null))
  (`SceneComponent.K2_AttachToComponent` (`Actor.RootComponent` _returnvalue) (`self.Mesh`) "spear_socket" "SnapToTarget" "SnapToTarget" "SnapToTarget" true))

(event `self.ReceiveTick`
  (params (DeltaSeconds :type "Float (single-precision)"))
  (`parent.ReceiveTick` DeltaSeconds))

(fn `UserConstructionScript`
  (`parent.UserConstructionScript`))